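; BP_ButtonStart is an interactable button that spawns a turtle at a linked Nest, labeled in-world with its NameButton text.
; Overlapping its Box enables player input on the actor, and leaving disables it.
; The first E press sets a one-shot flag, swaps the button material, and, if the Nest is valid, calls SpawnTurtle and plays a ribbon particle effect just above the nest.
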(event OnComponentBeginOverlap(Box)
  (params (OverlappedComponent :type Primitive%20Component%20Object%20Reference) (OtherActor :type Actor%20Object%20Reference) (OtherComp :type Primitive%20Component%20Object%20Reference) (OtherBodyIndex :type Integer) (bFromSweep :type Boolean) (SweepResult :type Hit%20Result%20Structure%20%28by%20ref%29))
  (Input|EnableInput (Game|GetPlayerController 0)))

(event OnComponentEndOverlap(Box)
  (params (OverlappedComponent :type Primitive%20Component%20Object%20Reference) (OtherActor :type Actor%20Object%20Reference) (OtherComp :type Primitive%20Component%20Object%20Reference) (OtherBodyIndex :type Integer))
  (Input|DisableInput (Game|GetPlayerController 0)))

(event EventBeginPlay
  (Rendering|Components|TextRender|SetText (Variables|Default|GetTextRender) (Variables|Default|GetNameButton)))

(event Collision|EventActorBeginOverlap
  (params (OtherActor :type Actor%20Object%20Reference)))

(event EventTick
  (params (DeltaSeconds :type Float%20%28single-precision%29)))

(event Input|KeyboardEvents|E
  (params (Key :type Key%20Structure :default "None"))
  (bind _nest (Variables|Default|GetNest))
  (:Pressed
    (if (not (Variables|Default|GetIsStartClicked))
      (Variables|Default|SetIsStartClicked true)
      (Rendering|Material|SetMaterial (Variables|Default|GetButton) 0 "/Game/StarterContent/Materials/M_AssetPlatform.M_AssetPlatform")
      ;[1 1 1] Spawn a turtle with effect spawning
      (Utilities|IsValid _nest
        (:Is%20Valid
          (Class|FTNest|SpawnTurtle _nest)
          (Niagara|SpawnSystematLocation "/Game/Turtle/VFX/RibbonSystemSpaw.RibbonSystemSpaw" (+ (Transformation|GetActorLocation _nest) "0, 0,40.000000")))))))

(fn ConstructionScript)